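; Loops and Lists demo Blueprint that shows several looping techniques on printed text and BP_Tree actors.
; BeginPlay starts an endless Delay-based loop and a while loop that prints a countdown in cycling colors.
; Each delayed pass calls an event that randomly yaws the next tree by stored index, resetting past the end.
; A ForEach event that rotates all trees at once is defined but not called here.
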(event `self.ReceiveBeginPlay`
  (`KismetSystemLibrary.PrintText` "Loops and Lists is Starting.")
  (`self.Simple Loop`)
  (`self.While Loop Function `))

(event `Simple Loop`
  (`KismetSystemLibrary.PrintText` "Inside Simple Loop, wait 3 seconds." :!label _label)
  (`self.LoopArrayOvetime`)
  (`KismetSystemLibrary.Delay` 3.0) ; Delay 2.833 secomds left.
  (goto _label))

(event `While Loop Function`
  (bind _colors (`self.Colors`))
  (while (> (`self.While Counter `) 0)
    (`KismetSystemLibrary.PrintText` (`|FormatText` "This is loop {count}. Ran after {seconds} seconds." (`self.While Counter `) (`KismetTextLibrary.Conv_DoubleToText` (`GameplayStatics.GetRealTimeSeconds`) "HalfToEven" false true 1 324 3)) true true (`|GetArrayItem` _colors (mod (`self.While Counter `) (`KismetArrayLibrary.Array_Length` _colors))) 20.0)
    (`/Engine/EditorBlueprintResources/StandardMacros.DecrementInt` (`self.While Counter `))))

(event `ChangeTreesForEach`
  (bind _outactors (`GameplayStatics.GetAllActorsOfClass` "/Game/BluePrint/BP_Tree.BP_Tree_C"))
  (for _array_element _outactors
    (`self.K2_SetActorRelativeRotation` _array_element (`KismetMathLibrary.MakeRotator` 0.0 0.0 (`KismetMathLibrary.RandomFloatInRange` 0.0 360.0)) false false))
  (`KismetSystemLibrary.PrintText` "Trees have been rotated"))

(event `LoopArrayOvetime`
  (bind _outactors (`GameplayStatics.GetAllActorsOfClass` "/Game/BluePrint/BP_Tree.BP_Tree_C"))
  (if (< (`self.OvertimeIndex`) (`KismetArrayLibrary.Array_Length` _outactors))
    (`self.K2_SetActorRelativeRotation` (`|GetArrayItem` _outactors (`self.OvertimeIndex`)) (`KismetMathLibrary.MakeRotator` 0.0 0.0 (`KismetMathLibrary.RandomFloatInRange` 0.0 360.0)) false false)
    (`/Engine/EditorBlueprintResources/StandardMacros.IncrementInt` (`self.OvertimeIndex`)
      (:`  `
        (`KismetSystemLibrary.Delay` 0.2)))
    (else
      (set `self.OvertimeIndex` 0) ; Rest index to zero
    )))

(fn `UserConstructionScript`)