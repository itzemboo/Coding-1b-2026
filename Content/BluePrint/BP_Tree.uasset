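; BP_Tree is a tree actor that picks a random static mesh on BeginPlay and is set up to grow in random increments.
; TheGrowLoop rolls a random step count and uses a DoN node, followed by a random delay, to call Grow, which adds to the mesh's relative scale.
; When the DoN counter matches the rolled count, the mesh switches to physics-only collision and prints a message.
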(event `self.ReceiveBeginPlay`
  (`StaticMeshComponent.SetStaticMesh` (`self.SM_Tree`) (`KismetArrayLibrary.Array_Random` (`self.New Mesh`)))
  (`self.The Grow Loop`))

(event `The Grow Loop`
  (bind _output_get (set `self.LoopCount` (`KismetMathLibrary.RandomIntegerInRange` 1 5)))
  (bind _counter (`/Engine/EditorBlueprintResources/StandardMacros.Do N` 0)
    (:`Exit`
      (`KismetSystemLibrary.Delay` (`KismetMathLibrary.RandomFloatInRange` 3.0 5.0))
      (`self.Grow`)
      (if (== _counter _output_get)
        (`PrimitiveComponent.SetCollisionEnabled` (`self.SM_Tree`) "PhysicsOnly")
        (`KismetSystemLibrary.PrintText` "Collision enabled ")))))

(event `Grow`
  (bind _sm_tree (`self.SM_Tree`))
  (`SceneComponent.SetRelativeScale3D` _sm_tree (+ (`SceneComponent.RelativeScale3D` _sm_tree) (`KismetMathLibrary.RandomFloatInRange` 0.2 0.4))))

(fn `UserConstructionScript`)