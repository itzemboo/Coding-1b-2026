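; BP_Door is a locked door that opens when a player carrying a key touches it.
; On overlap with a BP_ThirdPersonCharacter it prints a knocking message and checks the character's TotalKeys count.
; With a key, it spends one and destroys the door mesh and overlap box, so the opening is permanent; otherwise it prints that the door is locked.
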(event `self.ReceiveActorBeginOverlap`
  (params (OtherActor :type "Actor Object Reference"))
  (bind _asbp_third_person_character (cast `/Game/ThirdPerson/Blueprints/BP_ThirdPersonCharacter` OtherActor))
  (`KismetSystemLibrary.PrintText` "Player is knocking!")
  (bind _totalkeys (`/Game/ThirdPerson/Blueprints/BP_ThirdPersonCharacter.TotalKeys` _asbp_third_person_character))
  (if (> _totalkeys 0)
    (`/Engine/EditorBlueprintResources/StandardMacros.DecrementInt` _totalkeys
      (:`  `
        (`ActorComponent.K2_DestroyComponent` (`self.SM_Bld_Door_01`))
        (`ActorComponent.K2_DestroyComponent` (`self.OverLapBox`))))
    (else
      (`KismetSystemLibrary.PrintText` "I am Locked!"))))

(fn `UserConstructionScript`)